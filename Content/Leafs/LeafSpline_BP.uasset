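; Procedural leaf actor that builds a randomized leaf outline and its veins at BeginPlay.
; A seeded stream jitters points along a width profile from base through middle to tip, laid forward on one side and back on the other as a closed spline.
; PCG generates from that outline, then spawned LeafVein_BP actors run PCG along splines from the base midpoint to the tip and to random outline points.
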(event EventBeginPlay
  (bind _pcg (Variables|Default|GetPCG))
  (bind _numofpoints (Variables|Default|GetNumOfPoints))
  (bind _splineleaf (Variables|Default|GetSplineLeaf))
  (bind _splineleaf_2 (Variables|Default|GetSplineLeaf))
  (bind _numofpoints_2 (Variables|Default|GetNumOfPoints))
  (bind _numofpoints_3 (Variables|Default|GetNumOfPoints))
  (bind _sharpness (Variables|Default|GetSharpness))
  (bind _sharpness_2 (Variables|Default|GetSharpness))
  (bind _returnvalue (- _numofpoints_2 1))
  (bind _returnvalue_2 (- _numofpoints_3 1))
  (if (>= (Variables|Default|GetNew%20Seed) 0)
    _
    (else
      (bind _output_get (Variables|Default|SetNew%20Seed (Math|Random|RandomIntegerinRange 1 1000)))))
  (Math|Random|SetRandomStreamSeed (Variables|Default|GetStream) _output_get)
  (Spline|ClearSplinePoints (Variables|Default|GetSplineLeaf) true)
  (if (> (Variables|Default|GetMaxWidth) 0)
    _
    (else
      (Variables|Default|SetMaxWidth (/ (Variables|Default|GetNumOfPoints) 2))))
  (for _index (range 0 _returnvalue_2)
    (bind _output_get_2 (Variables|Default|SetProgress (/ (Math|Conversions|ToFloat(Integer) _index) (Math|Conversions|ToFloat(Integer) _returnvalue_2))))
    (Variables|Default|SetX_POS (* _output_get_2 (Variables|Default|GetLeafLength)))
    (Variables|Default|SetY_POS (Math|Float|Lerp (Variables|Default|GetBaseWidth) (Variables|Default|GetMidWidth) (Math|Trig|Sin(Radians) (* (Variables|Default|GetProgress) (Math|Trig|GetPI)))))
    (if (> _index (Variables|Default|GetMaxWidth))
      (bind _output_get_3 (Variables|Default|SetY_POS (Math|Float|Lerp (Variables|Default|GetMidWidth) (Variables|Default|GetTipWidth) (* (- (Variables|Default|GetProgress) 0.5) 2.0))))
      (bind _output_get_4 (Variables|Default|SetX_POS (+ (Variables|Default|GetX_POS) (* (Math|Trig|Sin(Radians) (* (- (Variables|Default|GetProgress) 0.5) (Math|Trig|GetPI))) 5e+01)))))
    (bind _output_get_5 (Variables|Default|SetY_POS_L (+ (* _output_get_3 -1.0) (Math|Random|RandomFloatinRangefromStream (Variables|Default|GetStream) (* _sharpness -1.0) _sharpness))))
    (Spline|AddSplinePoint (Variables|Default|GetSplineLeaf) (Math|Vector|MakeVector _output_get_4 _output_get_5 0.0) "Local" true))
  (bind _index_2 (Utilities|ReverseforLoop _returnvalue)
    (:Loop%20Body
      (bind _output_get_6 (Variables|Default|SetProgress (/ (Math|Conversions|ToFloat(Integer) _index_2) (Math|Conversions|ToFloat(Integer) _returnvalue))))
      (Variables|Default|SetX_POS (* _output_get_6 (Variables|Default|GetLeafLength)))
      (Variables|Default|SetY_POS (Math|Float|Lerp (Variables|Default|GetBaseWidth) (Variables|Default|GetMidWidth) (Math|Trig|Sin(Radians) (* (Variables|Default|GetProgress) (Math|Trig|GetPI)))))
      (if (> _index_2 (Variables|Default|GetMaxWidth))
        (bind _output_get_7 (Variables|Default|SetY_POS (Math|Float|Lerp (Variables|Default|GetMidWidth) (Variables|Default|GetTipWidth) (* (- (Variables|Default|GetProgress) 0.5) 2.0))))
        (bind _output_get_8 (Variables|Default|SetX_POS (+ (Variables|Default|GetX_POS) (* (Math|Trig|Sin(Radians) (* (- (Variables|Default|GetProgress) 0.5) (Math|Trig|GetPI))) 5e+01)))))
      (bind _output_get_9 (Variables|Default|SetY_POS_R (+ _output_get_7 (Math|Random|RandomFloatinRangefromStream (Variables|Default|GetStream) (* _sharpness_2 -1.0) _sharpness_2))))
      (Spline|AddSplinePoint (Variables|Default|GetSplineLeaf) (Math|Vector|MakeVector _output_get_8 _output_get_9 0.0) "Local" true))
    (:Completed
      (Spline|SetClosedLoop (Variables|Default|GetSplineLeaf) true true)
      (Class|PCGComponent|GenerateLocal _pcg true)
      (Class|PCGComponent|ClearPCGLink _pcg 0)
      (Development|PrintString "1. done")
      (Variables|Default|SetStartLocation (/ (+ (Spline|GetLocationatSplinePoint _splineleaf 0 "World") (Spline|GetLocationatSplinePoint _splineleaf (- (* (Variables|Default|GetNumOfPoints) 2) 1) "World")) "2.000000,2.000000,2.000000"))
      (bind _returnvalue_3 (Game|SpawnActorfromClass "/Game/Leafs/LeafVein_BP.LeafVein_BP_C" (Math|Transform|MakeTransform "0.000000,0.000000,2.000000" "0, 0, 0" "1.000000,1.000000,1.000000") "Undefined" "MultiplyWithRoot" 0 0))
      (Spline|SetLocationatSplinePoint (Variables|/Game/Leafs/LeafVein_BP.LeafVein_BP_C|GetSplineVein _returnvalue_3) 0 (Variables|Default|GetStartLocation) "World" true)
      (Spline|AddSplinePoint (Variables|/Game/Leafs/LeafVein_BP.LeafVein_BP_C|GetSplineVein _returnvalue_3) (/ (+ (Spline|GetLocationatSplinePoint _splineleaf_2 _numofpoints "World") (Spline|GetLocationatSplinePoint _splineleaf_2 (- _numofpoints 1) "World")) "2.000000,2.000000,2.000000") "World" true)
      (PCG|Generate (Variables|/Game/Leafs/LeafVein_BP.LeafVein_BP_C|GetPCG _returnvalue_3) true)
      (Development|PrintString "2. done")
      (for _index_3 (range 0 11)
        (bind _returnvalue_4 (Game|SpawnActorfromClass "/Game/Leafs/LeafVein_BP.LeafVein_BP_C" (Math|Transform|MakeTransform "0.000000,0.000000,2.000000" "0, 0, 0" "1.000000,1.000000,1.000000") "Undefined" "MultiplyWithRoot" 0 0))
        (Spline|SetLocationatSplinePoint (Variables|/Game/Leafs/LeafVein_BP.LeafVein_BP_C|GetSplineVein _returnvalue_4) 0 (Variables|Default|GetStartLocation) "World" true)
        (Spline|AddSplinePoint (Variables|/Game/Leafs/LeafVein_BP.LeafVein_BP_C|GetSplineVein _returnvalue_4) (Spline|GetLocationatSplinePoint (Variables|Default|GetSplineLeaf) (Math|Random|RandomIntegerinRangefromStream (Variables|Default|GetStream) 4 (- (* (Variables|Default|GetNumOfPoints) 2) 4)) "World") "World" true)
        (PCG|Generate (Variables|/Game/Leafs/LeafVein_BP.LeafVein_BP_C|GetPCG _returnvalue_4) true))
      (Development|PrintString "3. done"))))

(event Collision|EventActorBeginOverlap
  (params (OtherActor :type Actor%20Object%20Reference)))

(event EventTick
  (params (DeltaSeconds :type Float%20%28single-precision%29)))

(fn ConstructionScript)